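; GM_Testing is the testing game mode for a spell game, handling player numbering, respawning and match end.
; PostLogin numbers each PS_Testing by join order, and RespawnRequested spawns a BP_SpellGameCharacter on the authority, possessing it after a short delay.
; It exposes lookups into a total spell list.
; EndGame prints the winning player and restarts the game on a timer.
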(event Custom|RespawnRequested
  (params (Player :type PC%20Spell%20Object%20Reference) (Location :type Transform))
  (Utilities|IsValid Player
    (:Is%20Valid
      (Networking|SwitchHasAuthority
        (:Authority
          (bind _returnvalue (Game|SpawnActorfromClass "/Game/Blueprints/Player/BP_SpellGameCharacter.BP_SpellGameCharacter_C" Location "Undefined" "MultiplyWithRoot" 0 0))
          (Utilities|FlowControl|Delay 0.2)
          (Pawn|Possess Player _returnvalue))))))

(event EventPostLogin
  (params (NewPlayer :type Player%20Controller%20Object%20Reference))
  (bind _result (Math|Integer|IncrementInt (Variables|Default|GetPlayerCount))
    (:%20%20
      (bind _output_get (Variables|Default|SetPlayerCount _result))
      (bind _asps_testing (Utilities|Casting|CastToPS_Testing (Variables|/Script/Engine.Controller|GetPlayerState NewPlayer)))
      (Variables|/Game/Blueprints/GameMode/PS_Testing.PS_Testing_C|SetPlayerNumber _asps_testing _output_get))))

(event EventTick
  (params (DeltaSeconds :type Float%20%28single-precision%29)))

(fn ConstructionScript)

(fn GetCurrentSpelllist
  (params (SpellIndex :type Integer))
  (bind _totalspelllist (Variables|Default|GetTotalSpellList))
  (if (Utilities|Array|IsValidIndex _totalspelllist SpellIndex)
    (return (Utilities|Array|Get(acopy) _totalspelllist SpellIndex))))

(fn EndGame
  (params (Winner :type Integer))
  (Development|PrintString (Utilities|String|ToString(Integer) Winner) true true "(R=1.000000,G=0.067061,B=0.000000,A=1.000000)" 2e+01)
  (Development|PrintString "The winner is player:" true true "(R=1.000000,G=0.067061,B=0.000000,A=1.000000)" 2e+01)
  (Utilities|Time|SetTimerbyFunctionName 0 "Restart" 1e+01))

(fn GetCurrentSpellListLength
  (return (Utilities|Array|Length (Variables|Default|GetTotalSpellList))))

(fn Restart
  (bind _asgame_mode (Utilities|Casting|CastToGameMode (Game|GetGameMode)))
  (Class|GameMode|RestartGame _asgame_mode))