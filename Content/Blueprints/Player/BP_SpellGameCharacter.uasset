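; Player character Blueprint for a spell-casting game, handling death, respawn and spell swapping.
; On death the mesh ragdolls and movement stops; the server credits the killer's PS_Testing with a kill and starts a respawn timer.
; Respawn picks a random BP_SpawnPoint and, only if locally controlled, has player controller 0 respawn the pawn and unpossess.
; An authority-only function sets the WandComponent's spell class and constructs the new spell.
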(event Custom|RespawnSpellCharacter
  (bind _outactors (Actor|GetAllActorsOfClass "/Game/Blueprints/BP_SpawnPoint.BP_SpawnPoint_C"))
  (Variables|Default|SetActorTranform (Math|Transform|MakeTransform (.Location (Math|Transform|BreakTransform (Transformation|GetActorTransform (.OutItem (Utilities|Array|Random _outactors))))) (.Rotation (Math|Transform|BreakTransform (Variables|Default|GetActorTranform))) (.Scale (Math|Transform|BreakTransform (Variables|Default|GetActorTranform)))))
  (bind _aspc_spell (Utilities|Casting|CastToPC_Spell (Game|GetPlayerController 0)))
  (if (Pawn|IsLocallyControlled)
    (Default|RespawnPawn _aspc_spell (Variables|Default|GetActorTranform))
    (Pawn|UnPossess _aspc_spell)))

(event EventOnDeath
  (params (Killer :type Spell%20Game%20Character%20Object%20Reference))
  (bind _mesh (Variables|Character|GetMesh))
  (Collision|SetCollisionEnabled _mesh "PhysicsOnly")
  (Collision|SetCollisionObjectType _mesh "ECC_PhysicsBody")
  (Physics|SetSimulatePhysics _mesh true)
  (Collision|SetCollisionEnabled (Variables|Default|GetCapsuleComponent) "NoCollision")
  (Pawn|Components|CharacterMovement|DisableMovement (Variables|Default|GetSpellGameMovementComponent))
  (Networking|SwitchHasAuthority
    (:Authority
      (Utilities|Time|SetTimerbyEvent (delegate Custom|RespawnSpellCharacter) 5.0)
      (bind _asps_testing (Utilities|Casting|CastToPS_Testing (Variables|/Script/Engine.Pawn|GetPlayerState Killer)))
      (Default|ServerAddKill _asps_testing))))

(fn ConstructionScript)

(fn ChangeSpellbyClassonCharacter
  (params (NewSpell :type Spell%20Class%20Reference))
  (bind _wandcomponent (Variables|Default|GetWandComponent))
  (if (Ability|HasAuthority)
    (bind _output_get (Variables|/Script/Term4_Final.WandComponent|SetEquippedSpellClass _wandcomponent NewSpell))
    (Development|PrintString (Utilities|GetClassDisplayName (Variables|/Script/Term4_Final.WandComponent|GetEquippedSpellClass _wandcomponent)) true true "(R=0.000000,G=0.000000,B=0.000000,A=1.000000)")
    (bind _returnvalue (Game|ConstructObjectfromClass _output_get))
    (Variables|/Script/Term4_Final.WandComponent|SetEquippedSpell _wandcomponent _returnvalue)))